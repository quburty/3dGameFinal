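; BP_CEnemy is an enemy Blueprint that flashes its body red when hit.
; On BeginPlay it creates a dynamic material instance from the mesh's second material slot.
; The Hitted override calls the parent's logic, sets the BodyColor parameter to red, then uses a one-shot timer to restore it to white half a second later.
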(event `self.ReceiveBeginPlay`
  (bind _mesh (`self.Mesh`))
  (bind _returnvalue (`PrimitiveComponent.CreateDynamicMaterialInstance` _mesh 1 (`PrimitiveComponent.GetMaterial` _mesh 1) "None"))
  (set `self.Material` _returnvalue))

(event `self.Hitted`
  (`parent.Hitted`)
  (`MaterialInstanceDynamic.SetVectorParameterValue` (`self.Material`) "BodyColor" (struct :`R` 1.0 :`A` 1.0))
  (`KismetSystemLibrary.K2_SetTimerDelegate` (delegate `RestoreColor`) 0.5))

(event `RestoreColor`
  (`MaterialInstanceDynamic.SetVectorParameterValue` (`self.Material`) "BodyColor" (struct :`R` 1.0 :`G` 1.0 :`B` 1.0 :`A` 1.0)))

(fn `UserConstructionScript`)