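; Boss enemy Blueprint that triggers a phase change with a cinematic and swaps particle effects on its mesh.
; Start calls PhaseChange, then creates a player for the Master level sequence and plays it.
; Two emitter events share one Particle reference: the first attaches a heal aura, and the second destroys it and attaches a magic circle.
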(event `self.ReceiveBeginPlay`)

(event `Start`
  (`self.PhaseChange`)
  (bind (_outactor _returnvalue) (`LevelSequencePlayer.CreateLevelSequencePlayer` "/Game/Cinematics/Master.Master"))
  (`MovieSceneSequencePlayer.Play` _returnvalue))

(event `SpawnEmitter1`
  (bind _returnvalue (`GameplayStatics.SpawnEmitterAttached` "/Game/Effects/FXVarietyPack/Particles/P_ky_healAura.P_ky_healAura" (`self.Mesh`)))
  (set `self.Particle` _returnvalue))

(event `SpawnEmitter2`
  (`ActorComponent.K2_DestroyComponent` (`self.Particle`))
  (bind _returnvalue (`GameplayStatics.SpawnEmitterAttached` "/Game/Effects/FXVarietyPack/Particles/P_ky_magicCircle1.P_ky_magicCircle1" (`self.Mesh`)))
  (set `self.Particle` _returnvalue))

(fn `UserConstructionScript`)