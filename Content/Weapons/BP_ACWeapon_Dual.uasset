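; BP_ACWeapon_Dual is a dual-wield weapon Blueprint that moves a main and a sub weapon between the owner character's hands and holsters.
; GrabWeapon attaches both components to their hand sockets on the character's mesh, and UngrabWeapon attaches them to their dual holster sockets.
; Every attachment uses KeepRelative rules, so each component's relative transform carries over to the new socket.
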(event `self.GrabWeapon`
  (bind _mesh (`Character.Mesh` (`self.GetOwnerCharacter`)))
  (`SceneComponent.K2_AttachToComponent` (`self.MainWeapon`) _mesh "Hand_Weapon" "KeepRelative" "KeepRelative" "KeepRelative" true)
  (`SceneComponent.K2_AttachToComponent` (`self.SubWeapon`) _mesh "Hand_SubWeapon" "KeepRelative" "KeepRelative" "KeepRelative" true))

(event `self.UngrabWeapon`
  (bind _mesh (`Character.Mesh` (`self.GetOwnerCharacter`)))
  (`SceneComponent.K2_AttachToComponent` (`self.MainWeapon`) _mesh "Holster_Dual" "KeepRelative" "KeepRelative" "KeepRelative" true)
  (`SceneComponent.K2_AttachToComponent` (`self.SubWeapon`) _mesh "Holster_Dual_SubWeapon" "KeepRelative" "KeepRelative" "KeepRelative" true))

(fn `UserConstructionScript`)