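; BP_ACWeapon_Sword is a sword-and-shield weapon that moves between the owning character's hands and holsters.
; GrabWeapon attaches the Sword and Shield components to the hand sockets on the character mesh.
; UngrabWeapon reattaches both to their holster sockets, keeping relative transforms in either case.
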(event `self.GrabWeapon`
  (bind _mesh (`Character.Mesh` (`self.GetOwnerCharacter`)))
  (`SceneComponent.K2_AttachToComponent` (`self.Sword`) _mesh "Hand_Weapon" "KeepRelative" "KeepRelative" "KeepRelative" true)
  (`SceneComponent.K2_AttachToComponent` (`self.Shield`) _mesh "Hand_Shield" "KeepRelative" "KeepRelative" "KeepRelative" true))

(event `self.UngrabWeapon`
  (bind _mesh (`Character.Mesh` (`self.GetOwnerCharacter`)))
  (`SceneComponent.K2_AttachToComponent` (`self.Sword`) _mesh "Holster_Sword" "KeepRelative" "KeepRelative" "KeepRelative" true)
  (`SceneComponent.K2_AttachToComponent` (`self.Shield`) _mesh "Holster_Shield" "KeepRelative" "KeepRelative" "KeepRelative" true))

(fn `UserConstructionScript`)